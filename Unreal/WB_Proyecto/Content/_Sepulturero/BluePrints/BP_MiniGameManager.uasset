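; BP_MiniGameManager handles the end of a minigame, granting its reward and returning the player to the main game level.
; WinMiniGame sets the GameInstance flag for the given reward (Ganxo, Dron or Gema), then calls ReturnHome, while GameOver returns without a reward.
; ReturnHome marks the return from a minigame in BP_GameInstance and opens its stored CurrentLevel.
; A debug key triggers an instant win with a debug reward.
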(event Custom|WinMiniGame
  (params (Reward :type String))
  (bind _gameinstance (Variables|Default|GetGameInstance))
  ;[1 1 1] Llamar a esta función cuando se gane el juego, especificad la recompensa.
  (Development|PrintString "Minijuego Completado")
  (switch string Reward
    (:Ganxo
      (Variables|/Game/_Sepulturero/BluePrints/BP_GameInstance.BP_GameInstance_C|SetGanxo _gameinstance true))
    (:Dron
      (Variables|/Game/_Sepulturero/BluePrints/BP_GameInstance.BP_GameInstance_C|SetDron _gameinstance true))
    (:Gema
      (Variables|/Game/_Sepulturero/BluePrints/BP_GameInstance.BP_GameInstance_C|SetGema _gameinstance true)))
  (CallFunction|ReturnHome))

(event Custom|ReturnHome
  (bind _gameinstance (Variables|Default|GetGameInstance))
  ;[1 1 1] Llamar a esta función si se requiere volver a la sala del juego principal.
  (Variables|/Game/_Sepulturero/BluePrints/BP_GameInstance.BP_GameInstance_C|SetreturnsFromMinigame _gameinstance true)
  (Game|OpenLevel(byName) (Variables|/Game/_Sepulturero/BluePrints/BP_GameInstance.BP_GameInstance_C|GetCurrentLevel _gameinstance)))

(event Custom|GameOver
  ;[1 1 1] Llamar a esta función cuando se pierda el minijuego.
  (CallFunction|ReturnHome))

(event EventBeginPlay
  ;[1 1 1] BeginPlay donde recibe la referencia del GameInstance.
  (bind _asbp_game_instance (Utilities|Casting|CastToBP_GameInstance (Game|GetGameInstance)))
  (Variables|Default|SetGameInstance _asbp_game_instance))

(event Input|KeyboardEvents|<
  (params (Key :type Key%20Structure))
  ;[1 1 1] Key para ganar el minijuego.
  (:Pressed
    (Development|PrintString "Debug pressed")
    (CallFunction|WinMiniGame (Variables|Default|GetDEBUG_REWARD))))

(fn ConstructionScript)
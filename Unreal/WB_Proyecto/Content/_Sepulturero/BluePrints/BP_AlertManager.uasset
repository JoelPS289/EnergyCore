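; Alert manager actor that tracks an accumulating alert meter for the game.
; AddAlert adds a quantity to the meter and fires FullAlertEvent at a fixed threshold, though that event is currently empty.
; LoadAlert reads the meter from BP_GameInstance and SaveAlert writes it back, keeping the value outside the actor.
; The UpdateAlertManager function repeats the same write as SaveAlert.
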(event Custom|AddAlert
  (params (Quantity :type Float%20%28single-precision%29))
  ;[1 1 1] Añadir cantidad alerta
  (Development|PrintString "alert added")
  (Variables|Default|SetAlertMeter (+ Quantity (Variables|Default|GetAlertMeter)))
  (if (>= (Variables|Default|GetAlertMeter) 1e+02)
    (CallFunction|FullAlertEvent)))

(event Custom|SaveAlert
  (bind _asbp_game_instance (Utilities|Casting|CastToBP_GameInstance (Game|GetGameInstance)))
  (Variables|/Game/_Sepulturero/BluePrints/BP_GameInstance.BP_GameInstance_C|SetInstance%20Alert%20Meter _asbp_game_instance (Variables|Default|GetAlertMeter)))

(event Custom|FullAlertEvent)

(event Custom|LoadAlert
  (bind _asbp_game_instance (Utilities|Casting|CastToBP_GameInstance (Game|GetGameInstance)))
  (Variables|Default|SetAlertMeter (Variables|/Game/_Sepulturero/BluePrints/BP_GameInstance.BP_GameInstance_C|GetInstance%20Alert%20Meter _asbp_game_instance)))

(event EventBeginPlay)

(event EventTick
  (params (DeltaSeconds :type Float%20%28single-precision%29)))

(fn ConstructionScript)

(fn UpdateAlertManager
  (bind _asbp_game_instance (Utilities|Casting|CastToBP_GameInstance (Game|GetGameInstance)))
  (Variables|/Game/_Sepulturero/BluePrints/BP_GameInstance.BP_GameInstance_C|SetInstance%20Alert%20Meter _asbp_game_instance (Variables|Default|GetAlertMeter)))
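; Alert manager variant for minigames (Minijocs) that restores the alert state when play begins.
; On BeginPlay it finds the first BP_AlertManager actor in the level and calls its LoadAlert.
; FullAlertEvent only prints a debug message announcing that Pedro has arrived.
; Unconnected leftover nodes copy InstanceAlertMeter from BP_GameInstance and print AlertMeter, but never run.
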(event Custom|GetInstanceAlert
  (bind _returnvalue (Actor|GetActorOfClass "/Game/_Sepulturero/BluePrints/BP_AlertManager.BP_AlertManager_C"))
  (Default|LoadAlert _returnvalue))

(event EventBeginPlay
  (CallFunction|GetInstanceAlert))

(event EventTick
  (params (DeltaSeconds :type Float%20%28single-precision%29)))

(event EventFullAlertEvent
  (Development|PrintString "Pedro ya llegó"))

(fn ConstructionScript
  (|CallParentFunction))
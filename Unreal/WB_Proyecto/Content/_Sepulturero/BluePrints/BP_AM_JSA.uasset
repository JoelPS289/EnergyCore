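; BP_AM_JSA is a child Blueprint, apparently an alert manager for a minigame, that ends the game when alert reaches its maximum.
; FullAlertEvent prints a debug string, finds BP_MiniGameManager and calls GameOver, which the author's note describes as a sample for returning to the main game.
; AddAlert logs the incoming quantity but passes a constant zero to the parent implementation instead of that value.
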(event EventBeginPlay
  (|CallParentFunction) ; This node is disabled and will not be called.\nDrag off pins to build functionality.
)

(event EventTick
  (params (DeltaSeconds :type Float%20%28single-precision%29))
  (|CallParentFunction DeltaSeconds) ; This node is disabled and will not be called.\nDrag off pins to build functionality.
)

(event EventFullAlertEvent
  ;[1 1 1] Este Evento se dispara cuando la alerta llega al máximo.
  ;;[0 0.5572 1 1 14] He puesto estos nodos como muestra. Buscan el MiniGame Manager y le dicen que la partida se ha terminado, para cargar el Juego Principal de vuelta. - David.
  (Development|PrintString "quwe")
  (bind _returnvalue (Actor|GetActorOfClass "/Game/_Sepulturero/BluePrints/BP_MiniGameManager.BP_MiniGameManager_C"))
  (Default|GameOver _returnvalue))

(event EventAddAlert
  (params (Quantity :type Float%20%28single-precision%29))
  ;[1 1 1] Llamad el Evento ADD ALERT para subir el nivel de Alerta.
  (Development|PrintString (Utilities|String|Append "Alerta Añadida: " (Utilities|String|ToString(Float) Quantity)))
  (|CallParentFunction 0.0))

(fn ConstructionScript
  (|CallParentFunction))
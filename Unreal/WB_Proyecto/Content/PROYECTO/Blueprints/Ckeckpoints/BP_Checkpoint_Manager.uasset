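; BP_Checkpoint_Manager stores the player's current respawn checkpoint and returns the spider drone to it.
; On BeginPlay it records the player character's starting transform as the default checkpoint.
; SendCheckpoint replaces the stored transform and prints its location.
; Teleport&Healing casts the player to BP_SpiderDrone, restores its energy through RestaurarEnergia, then teleports it to the saved location and rotation.
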(event Custom|Send%20Checkpoint
  (params (Checkpoint_Transform :type Transform))
  ;[1 1 1] Set Checkpoint
  (bind _output_get (Variables|Default|SetCurrent_Checkpoint Checkpoint_Transform))
  (Development|PrintString (Utilities|String|ToString(Vector) (.Location (Math|Transform|BreakTransform _output_get)))))

(event Custom|Teleport%20&%20Healing
  (bind _returnvalue (Game|GetPlayerCharacter 0))
  (bind _current_checkpoint (Variables|Default|GetCurrent_Checkpoint))
  (bind (_location _rotation) (Math|Transform|BreakTransform _current_checkpoint))
  ;[1 1 1] Teleport & Healing
  (bind _asbp_spider_drone (Utilities|Casting|CastToBP_SpiderDrone _returnvalue))
  (Default|RestaurarEnergia _asbp_spider_drone)
  (Transformation|Teleport _returnvalue _location _rotation))

(event EventBeginPlay
  (bind _returnvalue (Game|GetPlayerCharacter 0))
  ;[1 1 1] Default Checkpoint
  (Utilities|IsValid _returnvalue
    (:Is%20Valid
      (Variables|Default|SetCurrent_Checkpoint (Transformation|GetActorTransform _returnvalue)))))

(fn ConstructionScript)
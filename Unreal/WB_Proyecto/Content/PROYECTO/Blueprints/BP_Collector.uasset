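; BP_Collector is an interactable key pickup for the player's spider drone that also restores its energy.
; A sphere trigger tracks whether a BP_SpiderDrone is inside, gating the Interaccionllaves event.
; On a valid interaction it calls the player drone's key counter and energy restore functions.
; It then destroys the sphere and zeroes the point light to deactivate itself, leaving the actor in the world.
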(event OnComponentBeginOverlap(Sphere)
  (params (OverlappedComponent :type Primitive%20Component%20Object%20Reference) (OtherActor :type Actor%20Object%20Reference) (OtherComp :type Primitive%20Component%20Object%20Reference) (OtherBodyIndex :type Integer) (bFromSweep :type Boolean) (SweepResult :type Hit%20Result%20Structure%20%28by%20ref%29))
  (Utilities|Casting|CastToBP_SpiderDrone OtherActor)
  (Variables|Default|SetInsideTrigger true))

(event OnComponentEndOverlap(Sphere)
  (params (OverlappedComponent :type Primitive%20Component%20Object%20Reference) (OtherActor :type Actor%20Object%20Reference) (OtherComp :type Primitive%20Component%20Object%20Reference) (OtherBodyIndex :type Integer))
  (Utilities|Casting|CastToBP_SpiderDrone OtherActor)
  (Variables|Default|SetInsideTrigger false))

(event Custom|Interaccion%20llaves
  (Development|PrintString "Interaccion llave")
  (bind _asbp_spider_drone (Utilities|Casting|CastToBP_SpiderDrone (Game|GetPlayerCharacter 0)))
  (if (Variables|Default|GetInsideTrigger)
    ;[1 1 1] Sumar llave, curar, desactivar
    (Default|ContadorDeLlaves _asbp_spider_drone)
    (Default|RestaurarEnergia _asbp_spider_drone)
    (Components|DestroyComponent (Variables|Default|GetSphere))
    (Rendering|Components|Light|SetIntensity (Variables|Default|GetPointLight) 0.0)))

(fn ConstructionScript)
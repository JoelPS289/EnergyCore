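; BP_Stalagtite is a falling stalactite hazard for the spider drone player.
; Any trigger overlap plays an explosion sound at the player, but only BP_SpiderDrone starts a delay before gravity is enabled on the Estalactita component.
; Hitting the drone applies damage and launches the player along a scaled offset away from the actor.
; Any hit spawns a crash effect and destroys the actor, with debug prints left in.
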(event OnComponentBeginOverlap(Trigger)
  (params (OverlappedComponent :type Primitive%20Component%20Object%20Reference) (OtherActor :type Actor%20Object%20Reference) (OtherComp :type Primitive%20Component%20Object%20Reference) (OtherBodyIndex :type Integer) (bFromSweep :type Boolean) (SweepResult :type Hit%20Result%20Structure%20%28by%20ref%29))
  (bind _estalactita (Variables|Default|GetEstalactita))
  (Audio|PlaySoundatLocation "/Game/StarterContent/Audio/Explosion_Cue.Explosion_Cue" (Transformation|GetActorLocation (Game|GetPlayerCharacter 0)) "0, 0, 0" 1.0 1.0 0.0 0 0 0)
  (Utilities|Casting|CastToBP_SpiderDrone OtherActor)
  (Utilities|FlowControl|Delay (Variables|Default|GetStalac%20Fall%20Delay))
  (Utilities|IsValid _estalactita
    (:Is%20Valid
      (Physics|SetEnableGravity _estalactita true))))

(event OnComponentHit(Estalactita)
  (params (HitComponent :type Primitive%20Component%20Object%20Reference) (OtherActor :type Actor%20Object%20Reference) (OtherComp :type Primitive%20Component%20Object%20Reference) (NormalImpulse :type Vector :default "0, 0, 0") (Hit :type Hit%20Result%20Structure%20%28by%20ref%29))
  (bind _returnvalue (Game|GetPlayerCharacter 0))
  (bind _returnvalue_2 (Transformation|GetActorLocation))
  (bind _returnvalue_3 (Transformation|GetActorLocation _returnvalue))
  (bind _returnvalue_4 (- _returnvalue_3 _returnvalue_2))
  (bind (_x _y _z) (Math|Vector|BreakVector _returnvalue_4))
  (Development|PrintString "Colisin")
  (bind _asbp_spider_drone (Utilities|Casting|CastToBP_SpiderDrone OtherActor)
    (:then
      (Game|Damage|ApplyDamage _asbp_spider_drone (Variables|Default|GetStalac%20Damage) 0 0)
      (Niagara|SpawnSystematLocation "/Game/PROYECTO/Particulas/PS_EC_Stalac_Crash.PS_EC_Stalac_Crash" (+ (Transformation|GetWorldLocation (Variables|Default|GetEstalactita)) "0, 0,-60.000000") "0, 0, 0" "0.500000,0.500000,0.500000")
      (Components|DestroyComponent (Variables|Default|GetEstalactita))
      ;[1 1 1] Tocar Player
      (bind _asbp_spider_drone_2 (Utilities|Casting|CastToBP_SpiderDrone (Game|GetPlayerCharacter 0)))
      (Character|LaunchCharacter _asbp_spider_drone_2 (Math|Vector|MakeVector (* _x 14.0) (* _y 14.0) (* _z 3.5)) true true))
    (:CastFailed
      (Niagara|SpawnSystematLocation "/Game/PROYECTO/Particulas/PS_EC_Stalac_Crash.PS_EC_Stalac_Crash" (+ (Transformation|GetWorldLocation (Variables|Default|GetEstalactita)) "0, 0,-60.000000") "0, 0, 0" "0.500000,0.500000,0.500000")
      ;[1 1 1] Tocar Suelo
      (Development|PrintString "GROUND HIT")))
  (Actor|DestroyActor))

(fn ConstructionScript)
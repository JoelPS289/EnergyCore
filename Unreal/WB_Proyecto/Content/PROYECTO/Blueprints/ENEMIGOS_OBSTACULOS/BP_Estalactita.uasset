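; BP_Estalactita is a stalactite hazard that falls when the player passes its trigger.
; A Player overlap on Trigger enables gravity after a delay, though the explosion sound plays at the player for any overlapping actor.
; Its collider damages anything tagged Player or Suelo (ground), spawns an explosion and destroys the stalactite.
; On player hits, it also launches BP_BolitaChar away from the actor's origin as knockback.
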(event OnComponentBeginOverlap(Trigger)
  (params (OverlappedComponent :type Primitive%20Component%20Object%20Reference) (OtherActor :type Actor%20Object%20Reference) (OtherComp :type Primitive%20Component%20Object%20Reference) (OtherBodyIndex :type Integer) (bFromSweep :type Boolean) (SweepResult :type Hit%20Result%20Structure%20%28by%20ref%29))
  (Audio|PlaySoundatLocation "/Game/StarterContent/Audio/Explosion_Cue.Explosion_Cue" (Transformation|GetActorLocation (Game|GetPlayerCharacter 0)) "0, 0, 0" 1.0 1.0 0.0 0 0 0)
  (if (Actor|ActorHasTag OtherActor "Player")
    (Utilities|FlowControl|Delay (Variables|Default|GetStalac%20Fall%20Delay))
    (Physics|SetEnableGravity (Variables|Default|GetEstalactita) true)))

(event OnComponentBeginOverlap(Estalac_collider)
  (params (OverlappedComponent :type Primitive%20Component%20Object%20Reference) (OtherActor :type Actor%20Object%20Reference) (OtherComp :type Primitive%20Component%20Object%20Reference) (OtherBodyIndex :type Integer) (bFromSweep :type Boolean) (SweepResult :type Hit%20Result%20Structure%20%28by%20ref%29))
  (bind _returnvalue (Game|GetPlayerCharacter 0))
  (bind _returnvalue_2 (Transformation|GetActorLocation))
  (bind _returnvalue_3 (Actor|ActorHasTag OtherActor "Suelo"))
  (bind _returnvalue_4 (Actor|ActorHasTag OtherActor "Player"))
  (bind _returnvalue_5 (Transformation|GetActorLocation _returnvalue))
  (bind _returnvalue_6 (- _returnvalue_5 _returnvalue_2))
  (bind (_x _y _z) (Math|Vector|BreakVector _returnvalue_6))
  (if (or _returnvalue_4 _returnvalue_3)
    (Game|Damage|ApplyDamage OtherActor (Variables|Default|GetStalac%20Damage) 0 0)
    (if _returnvalue_4
      (Effects|SpawnEmitteratLocation "/Game/StarterContent/Particles/P_Explosion.P_Explosion" (Transformation|GetWorldLocation (Variables|Default|GetEstalactita)))
      ;[1 1 1] Tocar Player
      (bind _asbp_bolita_char (Utilities|Casting|CastToBP_BolitaChar (Game|GetPlayerCharacter 0)))
      (Character|LaunchCharacter _asbp_bolita_char (Math|Vector|MakeVector (* _x 14.0) (* _y 14.0) (* _z 3.5)) true true)
      (Actor|DestroyActor)
      (Development|PrintString "PLAYER HIT")
      (else
        ;[1 1 1] Tocar Suelo
        (if _returnvalue_3
          (Effects|SpawnEmitteratLocation "/Game/StarterContent/Particles/P_Explosion.P_Explosion" (+ (Transformation|GetWorldLocation (Variables|Default|GetEstalactita)) "0, 0,-40.000000"))
          (Development|PrintString "GROUND HIT")
          (Actor|DestroyActor))))))

(fn ConstructionScript)
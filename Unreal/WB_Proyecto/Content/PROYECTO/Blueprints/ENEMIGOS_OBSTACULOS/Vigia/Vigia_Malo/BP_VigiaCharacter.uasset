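; BP_VigiaCharacter is an enemy watcher that patrols a route and respawns the player when they come too close.
; It loops through PatrolPointsArray with AI MoveTo and a short pause between points, printing debug positions; a failed move halts the patrol.
; Tick compares player distance against one of three radii chosen by the player's FlashArrayIndex, setting Killable so the following tick calls Respawn on BP_BolitaChar.
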(event Custom|PatrolToPoint
  (Development|PrintString (Utilities|String|ToString(Vector) (Transformation|GetActorLocation self)) true true "(R=0.000000,G=0.660000,B=1.000000,A=1.000000)" 1e+01)
  ;[1 1 1] Patrulladura
  (Development|PrintString (Utilities|String|ToString(Vector) (Transformation|GetActorLocation (Utilities|Array|Get(acopy) (Variables|Default|GetPatrolPointsArray) (Variables|Default|GetPatrolPointsIndex)))) true true "(R=0.000000,G=1.000000,B=0.081616,A=1.000000)" 1e+01)
  (AI|AIMoveTo self "0, 0, 0" (Utilities|Array|Get(acopy) (Variables|Default|GetPatrolPointsArray) (Variables|Default|GetPatrolPointsIndex)) 5.0 false
    (:OnSuccess
      ;;[1 1 1] Delay entre rutas
      (Utilities|FlowControl|Delay 1.0)
      (if (>= (Variables|Default|GetPatrolPointsIndex) (- (Utilities|Array|Length (Variables|Default|GetPatrolPointsArray)) 1))
        (Variables|Default|SetPatrolPointsIndex 0)
        (else
          (Math|Integer|IncrementInt (Variables|Default|GetPatrolPointsIndex)
            (:%20%20
              _))))
      (CallFunction|PatroltoPoint))
    (:OnFail
      (Development|PrintString "Fail" true true "(R=1.000000,G=0.000000,B=0.987921,A=1.000000)"))))

(event EventBeginPlay
  ;[1 1 1] Patrulladura
  (CallFunction|PatroltoPoint))

(event EventTick
  (params (DeltaSeconds :type Float%20%28single-precision%29))
  (bind _returnvalue (Game|Player|GetPlayerPawn 0))
  (bind _returnvalue_2 (Transformation|GetActorLocation))
  (bind _returnvalue_3 (Transformation|GetActorLocation _returnvalue))
  (bind _returnvalue_4 (Math|Vector|Distance(Vector) _returnvalue_3 _returnvalue_2))
  ;[1 1 1] Deteccion y muerte
  (if (Variables|Default|GetKillable)
    (Default|Respawn (stale _asbp_bolita_char))
    (Variables|Default|SetKillable false)
    (else
      (bind _asbp_bolita_char (Utilities|Casting|CastToBP_BolitaChar (Game|GetPlayerCharacter 0)))
      (if (Math|Boolean|ORBoolean (and (== (Variables|/Game/PROYECTO/Blueprints/BP_BolitaChar.BP_BolitaChar_C|GetFlashArrayIndex _asbp_bolita_char) 0) (<= _returnvalue_4 2.5e+02)) (and (== (Variables|/Game/PROYECTO/Blueprints/BP_BolitaChar.BP_BolitaChar_C|GetFlashArrayIndex _asbp_bolita_char) 1) (<= _returnvalue_4 4e+02)) (and (== (Variables|/Game/PROYECTO/Blueprints/BP_BolitaChar.BP_BolitaChar_C|GetFlashArrayIndex _asbp_bolita_char) 2) (<= _returnvalue_4 6e+02)))
        (Variables|Default|SetKillable true)))))

(fn ConstructionScript)
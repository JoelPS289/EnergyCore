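; Vigia enemy character that patrols and respawns the BP_BolitaChar player when the player comes within detection range.
; On BeginPlay it hands its patrol points to the AI_Vigia2 controller; its own route-cycling logic is left unconnected.
; Each Tick compares player distance against one of three radii chosen by the player's FlashArrayIndex.
; A hit sets Killable, which triggers the respawn on the following tick and then clears.
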(event EventBeginPlay
  ;[1 1 1] Patrulladura
  (bind _asai_vigia_2 (Utilities|Casting|CastToAI_Vigia2 (Pawn|GetController)))
  (Default|InitializeArray _asai_vigia_2 (Variables|Default|GetPatrolPointsArray)))

(event EventTick
  (params (DeltaSeconds :type Float%20%28single-precision%29))
  (bind _returnvalue (Game|Player|GetPlayerPawn 0))
  (bind _returnvalue_2 (Transformation|GetActorLocation))
  (bind _returnvalue_3 (Transformation|GetActorLocation _returnvalue))
  (bind _returnvalue_4 (Math|Vector|Distance(Vector) _returnvalue_3 _returnvalue_2))
  ;[1 1 1] Deteccion y muerte
  (if (Variables|Default|GetKillable)
    (Default|Respawn (stale _asbp_bolita_char))
    (Variables|Default|SetKillable false)
    (else
      (bind _asbp_bolita_char (Utilities|Casting|CastToBP_BolitaChar (Game|GetPlayerCharacter 0)))
      (if (Math|Boolean|ORBoolean (and (== (Variables|/Game/PROYECTO/Blueprints/BP_BolitaChar.BP_BolitaChar_C|GetFlashArrayIndex _asbp_bolita_char) 0) (<= _returnvalue_4 2.5e+02)) (and (== (Variables|/Game/PROYECTO/Blueprints/BP_BolitaChar.BP_BolitaChar_C|GetFlashArrayIndex _asbp_bolita_char) 1) (<= _returnvalue_4 4e+02)) (and (== (Variables|/Game/PROYECTO/Blueprints/BP_BolitaChar.BP_BolitaChar_C|GetFlashArrayIndex _asbp_bolita_char) 2) (<= _returnvalue_4 6e+02)))
        (Variables|Default|SetKillable true)))))

(fn ConstructionScript)
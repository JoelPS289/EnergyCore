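; BP_Watcher_Character is the Watcher enemy: it hands patrol points to its AI_Watcher controller and targets the spider drone player with lightning.
; Each tick sets Killable when the player is within a range chosen by the drone's FlashArrayIndex, clearing it beyond a larger cutoff.
; While Killable, TheEmperor aims a Niagara lightning effect at the player; the Respawn call is disconnected.
; ShootMontage plays a supplied animation montage.
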(event Custom|The%20Emperor
  (bind _niagara (Variables|Default|GetNiagara))
  (Components|Activation|Activate _niagara false)
  (Niagara|SetNiagaraVariable(Vector3) _niagara "Lightning_EndPoint" (Transformation|GetActorLocation (Game|GetPlayerCharacter 0))))

(event EventBeginPlay
  ;[1 1 1] Patrulladura
  (bind _asai_watcher (Utilities|Casting|CastToAI_Watcher (Pawn|GetController)))
  (Default|InitializeArray _asai_watcher (Variables|Default|GetPatrolPointsArray))
  (Components|Activation|Deactivate (Variables|Default|GetNiagara)))

(event EventTick
  (params (DeltaSeconds :type Float%20%28single-precision%29))
  (bind _returnvalue (Game|Player|GetPlayerPawn 0))
  (bind _returnvalue_2 (Transformation|GetActorLocation))
  (bind _returnvalue_3 (Game|GetPlayerCharacter 0))
  (bind _returnvalue_4 (Transformation|GetActorLocation _returnvalue))
  (bind _returnvalue_5 (Math|Vector|Distance(Vector) _returnvalue_4 _returnvalue_2))
  ;[1 1 1] Deteccion y muerte
  (Utilities|IsValid _returnvalue_3
    (:Is%20Valid
      (if (> (Math|Vector|Distance(Vector) (Transformation|GetActorLocation _returnvalue_3) (Transformation|GetActorLocation)) 1e+03)
        (Variables|Default|SetKillable false))
      (if (Variables|Default|GetKillable)
        (CallFunction|TheEmperor)
        (else
          (Components|Activation|Deactivate (Variables|Default|GetNiagara))))
      (bind _asbp_spider_drone (Utilities|Casting|CastToBP_SpiderDrone (Game|GetPlayerCharacter 0)))
      (if (Math|Boolean|ORBoolean (and (== (Variables|/Game/PROYECTO/Blueprints/BP_SpiderDrone.BP_SpiderDrone_C|GetFlashArrayIndex _asbp_spider_drone) 0) (<= _returnvalue_5 4e+02)) (and (== (Variables|/Game/PROYECTO/Blueprints/BP_SpiderDrone.BP_SpiderDrone_C|GetFlashArrayIndex _asbp_spider_drone) 1) (<= _returnvalue_5 6e+02)) (and (== (Variables|/Game/PROYECTO/Blueprints/BP_SpiderDrone.BP_SpiderDrone_C|GetFlashArrayIndex _asbp_spider_drone) 2) (<= _returnvalue_5 8e+02)))
        (Variables|Default|SetKillable true)))))

(fn ConstructionScript)

(fn ShootMontage
  (params (Montage :type Anim%20Montage%20Object%20Reference))
  (Development|PrintString "play montage")
  (bind _returnvalue (Animation|PlayAnimMontage Montage 1.0 "None"))
  (return _returnvalue))
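; Vigia enemy character that patrols and shows a lightning effect toward the player when they come within detection range.
; BeginPlay passes its patrol points to the AI_Vigia controller.
; Each tick, the player's FlashArrayIndex selects the distance that sets Killable, which clears only beyond a larger cutoff.
; While Killable, TheEmperor aims the Niagara lightning endpoint at the player; the player Respawn call is disconnected, so nothing kills.
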(event Custom|The%20Emperor
  (bind _niagara (Variables|Default|GetNiagara))
  (Components|Activation|Activate _niagara false)
  (Niagara|SetNiagaraVariable(Vector3) _niagara "Lightning_EP" (Transformation|GetActorLocation (Game|GetPlayerCharacter 0))))

(event EventBeginPlay
  ;[1 1 1] Patrulladura
  (bind _asai_vigia (Utilities|Casting|CastToAI_Vigia (Pawn|GetController)))
  (Default|InitializeArray _asai_vigia (Variables|Default|GetPatrolPointsArray))
  (Components|Activation|Deactivate (Variables|Default|GetNiagara)))

(event EventTick
  (params (DeltaSeconds :type Float%20%28single-precision%29))
  (bind _returnvalue (Game|Player|GetPlayerPawn 0))
  (bind _returnvalue_2 (Transformation|GetActorLocation))
  (bind _returnvalue_3 (Transformation|GetActorLocation _returnvalue))
  (bind _returnvalue_4 (Math|Vector|Distance(Vector) _returnvalue_3 _returnvalue_2))
  ;[1 1 1] Deteccion y muerte
  (if (> (Math|Vector|Distance(Vector) (Transformation|GetActorLocation (Game|GetPlayerCharacter 0)) (Transformation|GetActorLocation)) 1e+03)
    (Variables|Default|SetKillable false))
  (if (Variables|Default|GetKillable)
    (CallFunction|TheEmperor)
    (else
      (Components|Activation|Deactivate (Variables|Default|GetNiagara))))
  (bind _asbp_bolita_char (Utilities|Casting|CastToBP_BolitaChar (Game|GetPlayerCharacter 0)))
  (if (Math|Boolean|ORBoolean (and (== (Variables|/Game/PROYECTO/Blueprints/BP_BolitaChar.BP_BolitaChar_C|GetFlashArrayIndex _asbp_bolita_char) 0) (<= _returnvalue_4 4e+02)) (and (== (Variables|/Game/PROYECTO/Blueprints/BP_BolitaChar.BP_BolitaChar_C|GetFlashArrayIndex _asbp_bolita_char) 1) (<= _returnvalue_4 6e+02)) (and (== (Variables|/Game/PROYECTO/Blueprints/BP_BolitaChar.BP_BolitaChar_C|GetFlashArrayIndex _asbp_bolita_char) 2) (<= _returnvalue_4 8e+02)))
    (Variables|Default|SetKillable true)))

(fn ConstructionScript)
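; BP_WaterLeak is a leak that drips water drops at its own transform.
; Tick feeds a Delay of GotaSpawnRate, acting as a repeating timer that calls GoteraSpawn to spawn each BP_WaterDrop.
; When a drop overlaps the Suelo_gota component, a splash emitter spawns just below it and the drop is destroyed.
; The splash component is destroyed after a short delay.
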(event OnComponentBeginOverlap(Suelo_gota)
  (params (OverlappedComponent :type Primitive%20Component%20Object%20Reference) (OtherActor :type Actor%20Object%20Reference) (OtherComp :type Primitive%20Component%20Object%20Reference) (OtherBodyIndex :type Integer) (bFromSweep :type Boolean) (SweepResult :type Hit%20Result%20Structure%20%28by%20ref%29))
  (bind _asbp_water_drop (Utilities|Casting|CastToBP_WaterDrop OtherActor))
  (bind _returnvalue (Effects|SpawnEmitteratLocation "/Game/WaterMaterials/Particles/P_Water_Splashes.P_Water_Splashes" (+ (Transformation|GetActorLocation _asbp_water_drop) "0, 0,-40.000000")))
  (Actor|DestroyActor _asbp_water_drop)
  (Utilities|FlowControl|Delay 0.7)
  (Components|DestroyComponent _returnvalue))

(event Custom|GoteraSpawn
  (Game|SpawnActorfromClass "/Game/PROYECTO/Blueprints/ENEMIGOS_OBSTACULOS/BP_WaterDrop.BP_WaterDrop_C" (Transformation|GetActorTransform) "Undefined" 0 0))

(event EventTick
  (params (DeltaSeconds :type Float%20%28single-precision%29))
  (Utilities|FlowControl|Delay (Variables|Default|GetGota%20Spawn%20Rate))
  (CallFunction|GoteraSpawn))

(fn ConstructionScript)
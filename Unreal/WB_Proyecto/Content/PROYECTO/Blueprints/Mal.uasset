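; Mal is a pickup actor that registers a key and heals the player when touched.
; On Box overlap by an actor tagged Player, it calls ContadorDeLlaves on the ThirdPersonCharacter fetched as player 0.
; It then adds Curacion to CurrentEnergy, capped at a hardcoded maximum, refreshes the health bar through RecalcularBarraVida and destroys itself.
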(event OnComponentBeginOverlap(Box)
  (params (OverlappedComponent :type Primitive%20Component%20Object%20Reference) (OtherActor :type Actor%20Object%20Reference) (OtherComp :type Primitive%20Component%20Object%20Reference) (OtherBodyIndex :type Integer) (bFromSweep :type Boolean) (SweepResult :type Hit%20Result%20Structure%20%28by%20ref%29))
  (if (Actor|ActorHasTag OtherActor "Player")
    (bind _asthird_person_character (Utilities|Casting|CastToThirdPersonCharacter (Game|GetPlayerCharacter 0)))
    (Default|ContadorDeLlaves _asthird_person_character)
    ;[1 1 1] Curación
    (bind _asthird_person_character_2 (Utilities|Casting|CastToThirdPersonCharacter (Game|GetPlayerCharacter 0)))
    (if (<= (+ (Variables|/Game/PROYECTO/Blueprints/ThirdPersonCharacter.ThirdPersonCharacter_C|GetCurrentEnergy _asthird_person_character_2) (Variables|Default|GetCuracion)) 1e+02)
      (Variables|/Game/PROYECTO/Blueprints/ThirdPersonCharacter.ThirdPersonCharacter_C|SetCurrentEnergy _asthird_person_character_2 (+ (Variables|/Game/PROYECTO/Blueprints/ThirdPersonCharacter.ThirdPersonCharacter_C|GetCurrentEnergy _asthird_person_character_2) (Variables|Default|GetCuracion)))
      (else
        (Variables|/Game/PROYECTO/Blueprints/ThirdPersonCharacter.ThirdPersonCharacter_C|SetCurrentEnergy _asthird_person_character_2 1e+02)))
    (Default|RecalcularBarraVida _asthird_person_character_2)
    (Actor|DestroyActor)))

(fn ConstructionScript)
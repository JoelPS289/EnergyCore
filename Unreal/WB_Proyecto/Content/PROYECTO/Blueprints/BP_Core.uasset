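; BP_Core is the goal object that triggers the win once the spider drone player has collected three keys (NLlaves).
; Tick polls the key count and repeatedly calls LightsUp on the referenced BP_EasyLights while it equals three.
; Overlapping Sphere1 with three keys also lights up, reveals NSCore, displaces the referenced BP_CoreMass and spawns an explosion.
; After a short delay it opens the WhiteBox_SemiAbierto level.
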(event OnComponentBeginOverlap(Sphere1)
  (params (OverlappedComponent :type Primitive%20Component%20Object%20Reference) (OtherActor :type Actor%20Object%20Reference) (OtherComp :type Primitive%20Component%20Object%20Reference) (OtherBodyIndex :type Integer) (bFromSweep :type Boolean) (SweepResult :type Hit%20Result%20Structure%20%28by%20ref%29))
  (bind _asbp_spider_drone (Utilities|Casting|CastToBP_SpiderDrone (Game|GetPlayerCharacter 0)))
  (if (== (Variables|/Game/PROYECTO/Blueprints/BP_SpiderDrone.BP_SpiderDrone_C|GetN_Llaves _asbp_spider_drone) 3)
    (bind _asbp_easy_lights (Utilities|Casting|CastToBP_EasyLights (Variables|Default|GetCoreLightsRef)))
    (Default|LightsUp _asbp_easy_lights)
    (Development|SetHiddeninGame (Variables|Default|GetNS_Core) false false)
    (bind _asbp_core_mass (Utilities|Casting|CastToBP_CoreMass (Variables|Default|GetCore_ref)))
    (Default|CoreDisplace _asbp_core_mass)
    (Effects|SpawnEmitteratLocation "/Game/StarterContent/Particles/P_Explosion.P_Explosion" (Transformation|GetActorLocation) "0, 0, 0" "4.000000,4.000000,4.000000")
    (Utilities|FlowControl|Delay 4.0)
    ;[1 1 1] ESTO ES EL GANAR
    (Game|OpenLevel(byName) "WhiteBox_SemiAbierto")))

(event EventTick
  (params (DeltaSeconds :type Float%20%28single-precision%29))
  (bind _asbp_spider_drone (Utilities|Casting|CastToBP_SpiderDrone (Game|GetPlayerCharacter 0)))
  (if (== (Variables|/Game/PROYECTO/Blueprints/BP_SpiderDrone.BP_SpiderDrone_C|GetN_Llaves _asbp_spider_drone) 3)
    (bind _asbp_easy_lights (Utilities|Casting|CastToBP_EasyLights (Variables|Default|GetCoreLightsRef)))
    (Default|LightsUp _asbp_easy_lights)))

(fn ConstructionScript)
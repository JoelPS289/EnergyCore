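; BP_Nucleo is a core actor that acts as a key-gated transition to the WhiteBox_SemiAbierto level.
; When a Player-tagged actor overlaps Sphere1, it reads the key count (NLlaves) from the player's BP_BolitaChar.
; With exactly three keys, it spawns an enlarged explosion emitter at its location, then opens the level by name after a short delay.
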(event OnComponentBeginOverlap(Sphere1)
  (params (OverlappedComponent :type Primitive%20Component%20Object%20Reference) (OtherActor :type Actor%20Object%20Reference) (OtherComp :type Primitive%20Component%20Object%20Reference) (OtherBodyIndex :type Integer) (bFromSweep :type Boolean) (SweepResult :type Hit%20Result%20Structure%20%28by%20ref%29))
  (if (Actor|ActorHasTag OtherActor "Player")
    (bind _asbp_bolita_char (Utilities|Casting|CastToBP_BolitaChar (Game|GetPlayerCharacter 0)))
    (if (== (Variables|/Game/PROYECTO/Blueprints/BP_BolitaChar.BP_BolitaChar_C|GetN_Llaves _asbp_bolita_char) 3)
      (Effects|SpawnEmitteratLocation "/Game/StarterContent/Particles/P_Explosion.P_Explosion" (Transformation|GetActorLocation) "0, 0, 0" "4.000000,4.000000,4.000000")
      (Utilities|FlowControl|Delay 1.5)
      (Game|OpenLevel(byName) "WhiteBox_SemiAbierto"))))

(fn ConstructionScript)
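; BP_Recolectores is a key pickup for the BP_BolitaChar player character.
; Its Interaccionllaves event increments the character's key counter, restores energy, destroys the Sphere and sets the PointLight intensity to zero.
; Sphere overlaps maintain an InsideTrigger flag, but the branch that checks it is unconnected, so the interaction itself does not test proximity.
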(event OnComponentBeginOverlap(Sphere)
  (params (OverlappedComponent :type Primitive%20Component%20Object%20Reference) (OtherActor :type Actor%20Object%20Reference) (OtherComp :type Primitive%20Component%20Object%20Reference) (OtherBodyIndex :type Integer) (bFromSweep :type Boolean) (SweepResult :type Hit%20Result%20Structure%20%28by%20ref%29))
  (Utilities|Casting|CastToBP_BolitaChar OtherActor)
  (Variables|Default|SetInsideTrigger true))

(event OnComponentEndOverlap(Sphere)
  (params (OverlappedComponent :type Primitive%20Component%20Object%20Reference) (OtherActor :type Actor%20Object%20Reference) (OtherComp :type Primitive%20Component%20Object%20Reference) (OtherBodyIndex :type Integer))
  (Utilities|Casting|CastToBP_BolitaChar OtherActor)
  (Variables|Default|SetInsideTrigger false))

(event Custom|Interaccion%20llaves
  (Development|PrintString "Interaccion llave")
  (bind _asbp_bolita_char (Utilities|Casting|CastToBP_BolitaChar (Game|GetPlayerCharacter 0)))
  ;[1 1 1] Sumar llave, curar, desactivar
  (Default|ContadorDeLlaves _asbp_bolita_char)
  (Default|RestaurarEnergia _asbp_bolita_char)
  (Components|DestroyComponent (Variables|Default|GetSphere))
  (Rendering|Components|Light|SetIntensity (Variables|Default|GetPointLight) 0.0))

(fn ConstructionScript)